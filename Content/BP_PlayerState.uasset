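; BP_PlayerState is a player state that assigns a team and unit spawn point to players.
; On BeginPlay it loops over all BP_ThirdPersonCharacter actors, writing Team A or B and the matching spawn to each one's BP_PlayerState.
; The split compares each character to the player state itself, so the Team B branch appears unreachable.
; GetCurrentPlayerState repeats the loop, returning at the first character, provided its cast succeeds.
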(event EventBeginPlay
  (bind _outactors (Actor|GetAllActorsOfClass "/Game/ThirdPerson/Blueprints/BP_ThirdPersonCharacter.BP_ThirdPersonCharacter_C"))
  (for _array_element _outactors
    (if (!= _array_element self)
      (bind _asbp_player_state (Utilities|Casting|CastToBP_PlayerState (Variables|/Script/Engine.Pawn|GetPlayerState _array_element)))
      (Utilities|FlowControl|Sequence
        (:then_0
          (Variables|BP_PlayerState_C|SetTeam _asbp_player_state "A"))
        (:then_1
          (Variables|BP_PlayerState_C|SetUnitSpawnPoint _asbp_player_state (Variables|Default|GetTeamASpawn))))
      (else
        (bind _asbp_player_state_2 (Utilities|Casting|CastToBP_PlayerState (Variables|/Script/Engine.Pawn|GetPlayerState _array_element)))
        (Utilities|FlowControl|Sequence
          (:then_0
            (Variables|BP_PlayerState_C|SetUnitSpawnPoint _asbp_player_state_2 (Variables|Default|GetTeamBSpawn)))
          (:then_1
            (Variables|BP_PlayerState_C|SetTeam _asbp_player_state_2 "B")))))))

(fn ConstructionScript)

(fn GetCurrentPlayerState
  (bind _outactors (Actor|GetAllActorsOfClass "/Game/ThirdPerson/Blueprints/BP_ThirdPersonCharacter.BP_ThirdPersonCharacter_C"))
  (for _array_element _outactors
    (if (!= _array_element self)
      (Utilities|Casting|CastToBP_PlayerState (Variables|/Script/Engine.Pawn|GetPlayerState _array_element))
      (else
        (Utilities|Casting|CastToBP_PlayerState (Variables|/Script/Engine.Pawn|GetPlayerState _array_element))))
    (return 0 0)))